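; 빵빵이_BP is an NPC Blueprint that patrols a looping route through an array of target actors.
; On BeginPlay it calls PatrolPoint, which uses AI MoveTo to walk to the current target.
; On success it sets and prints Speed from the mesh forward vector's length, advances or wraps the index, and calls PatrolPoint again.
; A failed move is not handled, so the patrol stops there.
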(event Custom|PatrolPoint
  (AI|AIMoveTo self "0, 0, 0" (Utilities|Array|Get(acopy) (Variables|Default|GetTarget) (Variables|Default|GetTarget_Number)) 5.0 true
    (:OnSuccess
      (bind _output_get (Variables|Default|SetSpeed (* 100 (Math|Vector|VectorLength (Math|Vector|GetForwardVector (Variables|Character|GetMesh))))))
      (Development|PrintString (Utilities|String|ToString(Float) _output_get))
      (if (>= (Variables|Default|GetTarget_Number) (- (Utilities|Array|Length (Variables|Default|GetTarget)) 1))
        (Variables|Default|SetTarget_Number 0)
        (else
          (Math|Integer|IncrementInt (Variables|Default|GetTarget_Number)
            (:%20%20
              _))))
      (CallFunction|PatrolPoint))))

(event EventBeginPlay
  (CallFunction|PatrolPoint))

(fn ConstructionScript)