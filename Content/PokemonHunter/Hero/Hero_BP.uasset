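; Player hero character for PokemonHunter, with walking, jumping, sprinting and a toggleable bicycle ride.
; Movement axes follow control yaw, and holding right mouse swaps from the main camera to a secondary one.
; Key 2 flip-flops riding, changing bicycle visibility, mesh pose and animation mode, walk speed, and two temporary child actor components.
; The Ride flag selects which speeds Left Shift applies on press and release.
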(event Input|AxisEvents|InputAxisRight_input
  (params (AxisValue :type Float%20%28single-precision%29))
  (Pawn|Input|AddMovementInput (Math|Vector|GetRightVector (Math|Rotator|MakeRotator 0.0 0.0 (.yaw (Pawn|GetControlRotation :!class /Script/Engine.Pawn)))) AxisValue false))

(event Input|AxisEvents|InputAxisForward_input
  (params (AxisValue :type Float%20%28single-precision%29))
  (Pawn|Input|AddMovementInput (Math|Vector|GetForwardVector (Math|Rotator|MakeRotator 0.0 0.0 (.yaw (Pawn|GetControlRotation :!class /Script/Engine.Pawn)))) AxisValue false))

(event Input|KeyboardEvents|SpaceBar
  (params (Key :type Key%20Structure :default "None"))
  (:Pressed
    (Character|Jump)))

(event Input|KeyboardEvents|LeftShift
  (params (Key :type Key%20Structure :default "None"))
  (bind _charactermovement (Variables|Character|GetCharacterMovement))
  (:Pressed
    (if (Variables|Default|GetRide)
      (Variables|/Script/Engine.CharacterMovementComponent|SetMaxWalkSpeed _charactermovement 1.8e+03)
      (else
        (Variables|/Script/Engine.CharacterMovementComponent|SetMaxWalkSpeed _charactermovement 6e+02))))
  (:Released
    (if (Variables|Default|GetRide)
      (Variables|/Script/Engine.CharacterMovementComponent|SetMaxWalkSpeed _charactermovement 1.2e+03)
      (else
        (Variables|/Script/Engine.CharacterMovementComponent|SetMaxWalkSpeed _charactermovement 1.5e+02)))))

(event Input|MouseEvents|RightMouseButton
  (params (Key :type Key%20Structure :default "None"))
  (:Pressed
    (Components|Activation|Activate (Variables|Default|GetCamera) false)
    (Components|Activation|Deactivate (Variables|Default|GetMainCamera)))
  (:Released
    (Components|Activation|Activate (Variables|Default|GetMainCamera) false)
    (Components|Activation|Deactivate (Variables|Default|GetCamera))))

(event Input|KeyboardEvents|2
  (params (Key :type Key%20Structure :default "None"))
  (bind _mesh (Variables|Character|GetMesh))
  (bind _mesh_2 (Variables|Character|GetMesh))
  (:Pressed
    (Utilities|FlowControl|FlipFlop
      (:A
        (Variables|Default|SetRide true)
        (Rendering|SetVisibility (Variables|Default|GetBicycle) true false)
        (Components|Animation|PlayAnimation _mesh_2 "/Game/PokemonHunter/Hero/Animation/Flying_Bicycle_Kick.Flying_Bicycle_Kick" true)
        (Transformation|AddLocalRotation _mesh_2 "0, 0,45.000000" false false)
        (Transformation|AddLocalOffset _mesh_2 "0.000000,-45.000000,-18.000000" false false)
        (Variables|/Script/Engine.CharacterMovementComponent|SetMaxWalkSpeed (Variables|Character|GetCharacterMovement) 1.2e+03)
        (bind _returnvalue (AddComponent|AddChildActorComponent false))
        (bind _returnvalue_2 (AddComponent|AddChildActorComponent false)))
      (:B
        (Variables|Default|SetRide false)
        (Rendering|SetVisibility (Variables|Default|GetBicycle) false false)
        (Components|Animation|SetAnimationMode _mesh "AnimationBlueprint")
        (Transformation|AddLocalOffset _mesh "0.000000,45.000000,18.000000" false false)
        (Transformation|AddLocalRotation _mesh "0.000000,0.000000,-45.000000" false false)
        (Variables|/Script/Engine.CharacterMovementComponent|SetMaxWalkSpeed (Variables|Character|GetCharacterMovement) 1.5e+02)
        (Components|DestroyComponent _returnvalue)
        (Components|DestroyComponent _returnvalue_2)))))

(fn ConstructionScript)